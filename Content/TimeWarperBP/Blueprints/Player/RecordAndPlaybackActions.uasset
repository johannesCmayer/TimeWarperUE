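; Actor component that records and replays its owning first-person character's movement, camera pitch and projectile shots.
; While recording, Tick logs timestamped transforms and pitch, and RecordProjectile stores shot transforms and times.
; In playback, PlaybackLogic advances iterators against a timer, disables camera control rotation, sets recorded transforms and respawns projectiles with fire sound and animation.
; Record, Playback and Pause switch modes; PlaybackMovement is an uncalled variant of PlaybackLogic.
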(event `self.ReceiveBeginPlay`
  (bind _returnvalue (`self.GetOwner`))
  ;[1 1 1] Get Reffernces
  (set `self.MyParent` _returnvalue)
  (set `self.MyCamera` (`Actor.GetComponentByClass` _returnvalue "/Script/Engine.CameraComponent")))

(event `RecordProjectile`
  (params (Target :type "Actor Object Reference"))
  (`self.RecordSpawnedProjectile` Target))

(event `self.ReceiveTick`
  (params (DeltaSeconds :type "Float (single-precision)"))
  (if (`self.bRecord`)
    (`self.RecordMovement`)
    (elif (`self.bPlayback`)
      (`self.PlaybackLogic`))))

(fn `ClearRecordedData`
  (set `self.RecordingTimer` 0.0)
  (set `self.PlaybackTimer` 0.0)
  (`KismetArrayLibrary.Array_Clear` (`self.TimeStamps`))
  (`KismetArrayLibrary.Array_Clear` (`self.PositionsActor`))
  (`KismetArrayLibrary.Array_Clear` (`self.YRotationsCamera`))
  (set `self.MovementIterator` 0)
  (`KismetArrayLibrary.Array_Clear` (`self.SpawnPositionProjectile`))
  (`KismetArrayLibrary.Array_Clear` (`self.SpawnTimeProjectile`))
  (set `self.ProjectileItterator` 0))

(fn `Pause`
  (set `self.bPlayback` false)
  (set `self.bRecord` false))

(fn `Playback`
  (set `self.bPlayback` true)
  (set `self.bRecord` false))

(fn `PlaybackLogic`
  ;[1 1 1] Timer for playback
  (set `self.PlaybackTimer` (+ (`self.PlaybackTimer`) (`GameplayStatics.GetWorldDeltaSeconds`)))
  ;[0.5565 1 0.5248] Movement
  ;;[1 1 1] Check if entry at MovementItterator exists
  (if (and (!= (`KismetArrayLibrary.Array_Length` (`self.PositionsActor`)) 0) (< (`self.MovementIterator`) (`KismetArrayLibrary.Array_Length` (`self.PositionsActor`))))
    ;;[1 1 1] Set Camera to not use Pawn Control Rotation
    (if (`CameraComponent.bUsePawnControlRotation` (`self.MyCamera`))
      (set `CameraComponent.bUsePawnControlRotation` false (`self.MyCamera`)))
    ;;[1 1 1] Set actor transform
    (`Actor.K2_SetActorTransform` (`self.MyParent`) (`|GetArrayItem` (`self.PositionsActor`) (`self.MovementIterator`)) false false)
    ;;[1 1 1] Set camera YRot
    (`SceneComponent.K2_SetRelativeRotation` (`self.MyCamera`) (`KismetMathLibrary.MakeRotator` 0.0 (`|GetArrayItem` (`self.YRotationsCamera`) (`self.MovementIterator`))) false false)
    ;;[1 1 1] Increment MovementItterator when timestamp overpassed
    (while (and (>= (`self.PlaybackTimer`) (`|GetArrayItem` (`self.TimeStamps`) (`self.MovementIterator`))) (< (`self.MovementIterator`) (- (`KismetArrayLibrary.Array_Length` (`self.TimeStamps`)) 1)))
      (bind _result (`/Engine/EditorBlueprintResources/StandardMacros.IncrementInt` (`self.MovementIterator`))
        (:`  `
          (set `self.MovementIterator` _result))))
    ;[0.4998 1 0.5112] Projectiles
    ;;[1 1 1] Check if ProjectileIterator entry exists
    (if (and (> (`KismetArrayLibrary.Array_Length` (`self.SpawnTimeProjectile`)) 0) (< (`self.ProjectileItterator`) (`KismetArrayLibrary.Array_Length` (`self.SpawnPositionProjectile`))))
      ;;[1 1 1] Spawn Projectile if correct time
      (if (and (>= (`self.PlaybackTimer`) (`|GetArrayItem` (`self.SpawnTimeProjectile`) (`self.ProjectileItterator`))) (< (`self.ProjectileItterator`) (- (`KismetArrayLibrary.Array_Length` (`self.SpawnTimeProjectile`)) 1)))
        (`|SpawnActorFromClass` "/Game/TimeWarperBP/Blueprints/Player/FirstPersonProjectile.FirstPersonProjectile_C" (`|GetArrayItem` (`self.SpawnPositionProjectile`) (`self.ProjectileItterator`)) "AlwaysSpawn" "OverrideRootScale" null null) ; Spawn projectile
        ;;[1 1 1] Play firing sound and animation
        (bind _asfirst_person_character (cast `/Game/TimeWarperBP/Blueprints/Player/FirstPersonCharacter` (`self.MyParent`)))
        (`/Game/TimeWarperBP/Blueprints/Player/FirstPersonCharacter.PlayShootSound` _asfirst_person_character)
        (`/Game/TimeWarperBP/Blueprints/Player/FirstPersonCharacter.PlayFirstPersonShootAnimation` _asfirst_person_character)
        ;;[1 1 1] Increment ProjectileItterator
        (while (and (>= (`self.PlaybackTimer`) (`|GetArrayItem` (`self.SpawnTimeProjectile`) (`self.ProjectileItterator`))) (< (`self.ProjectileItterator`) (- (`KismetArrayLibrary.Array_Length` (`self.SpawnTimeProjectile`)) 1)))
          (bind _result_2 (`/Engine/EditorBlueprintResources/StandardMacros.IncrementInt` (`self.ProjectileItterator`))
            (:`  `
              (set `self.ProjectileItterator` _result_2))))))
    (else
      (`KismetSystemLibrary.PrintString` "NoMoreRecordedData"))))

(fn `PlaybackMovement`
  (bind _returnvalue (>= (`self.PlaybackTimer`) (`|GetArrayItem` (`self.TimeStamps`) (`self.MovementIterator`))))
  ;[0.5565 1 0.5248] Playback
  ;;[1 1 1] Check if entry at MovementItterator exists
  (if (and (!= (`KismetArrayLibrary.Array_Length` (`self.PositionsActor`)) 0) (< (`self.MovementIterator`) (`KismetArrayLibrary.Array_Length` (`self.PositionsActor`))))
    ;;[1 1 1] Set Camera to not use Pawn Control Rotation
    (if (`CameraComponent.bUsePawnControlRotation` (`self.MyCamera`))
      (set `CameraComponent.bUsePawnControlRotation` false (`self.MyCamera`)))
    ;;[1 1 1] Set actor transform
    (`Actor.K2_SetActorTransform` (`self.MyParent`) (`|GetArrayItem` (`self.PositionsActor`) (`self.MovementIterator`)) false false)
    ;;[1 1 1] Set camera YRot
    (`SceneComponent.K2_SetRelativeRotation` (`self.MyCamera`) (`KismetMathLibrary.MakeRotator` 0.0 (`|GetArrayItem` (`self.YRotationsCamera`) (`self.MovementIterator`))) false false)
    ;;[1 1 1] Increment MovementItterator when timestamp overpassed
    (if (not _returnvalue)
      (`KismetSystemLibrary.PrintString` (`KismetStringLibrary.Conv_BoolToString` _returnvalue)))
    (bind _result (`/Engine/EditorBlueprintResources/StandardMacros.IncrementInt` (`self.MovementIterator`))
      (:`  `
        (set `self.MovementIterator` _result)
        ;;[1 1 1] Check if ProjectileIterator entry exists
        (if (and (> (`KismetArrayLibrary.Array_Length` (`self.SpawnTimeProjectile`)) 0) (< (`self.ProjectileItterator`) (`KismetArrayLibrary.Array_Length` (`self.SpawnPositionProjectile`))))
          ;;[1 1 1] Spawn Projectile if correct time
          (if (>= (`self.PlaybackTimer`) (`|GetArrayItem` (`self.SpawnTimeProjectile`) (`self.ProjectileItterator`)))
            (`|SpawnActorFromClass` "/Game/TimeWarperBP/Blueprints/Player/FirstPersonProjectile.FirstPersonProjectile_C" (`|GetArrayItem` (`self.SpawnPositionProjectile`) (`self.ProjectileItterator`)) "AlwaysSpawn" "OverrideRootScale" null null) ; Spawn projectile
            ;;[1 1 1] Play firing sound and animation
            (bind _asfirst_person_character (cast `/Game/TimeWarperBP/Blueprints/Player/FirstPersonCharacter` (`self.MyParent`)))
            (`/Game/TimeWarperBP/Blueprints/Player/FirstPersonCharacter.PlayShootSound` _asfirst_person_character)
            (`/Game/TimeWarperBP/Blueprints/Player/FirstPersonCharacter.PlayFirstPersonShootAnimation` _asfirst_person_character)
            ;;[1 1 1] Increment ProjectileItterator
            (bind _result_2 (`/Engine/EditorBlueprintResources/StandardMacros.IncrementInt` (`self.ProjectileItterator`))
              (:`  `
                (set `self.ProjectileItterator` _result_2)))))))
    (else
      (`KismetSystemLibrary.PrintString` "NoMoreRecordedData"))))

(fn `PlayFromBegining`
  (`self.ResetPlaybackToBegining`)
  (`self.Playback`))

(fn `Record`
  (set `self.bPlayback` false)
  (set `self.bRecord` true))

(fn `RecordMovement`
  ;[1 1 1] Set Camera to use Pawn Control Rotation
  (if (not (`CameraComponent.bUsePawnControlRotation` (`self.MyCamera`)))
    (set `CameraComponent.bUsePawnControlRotation` true (`self.MyCamera`))
    (else
      ;[1 1 1] Timer for recording
      (bind _output_get (set `self.RecordingTimer` (+ (`self.RecordingTimer`) (`GameplayStatics.GetWorldDeltaSeconds`))))
      ;[1 1 1] Record Time
      (`KismetArrayLibrary.Array_Add` (`self.TimeStamps`) _output_get)
      ;[1 1 1] RecordMovement
      ;;[1 1 1] Record Actor Transform
      (`KismetArrayLibrary.Array_Add` (`self.PositionsActor`) (`Actor.GetTransform` (`self.MyParent`)))
      ;;[1 1 1] Record Camera YRot
      (`KismetArrayLibrary.Array_Add` (`self.YRotationsCamera`) (.pitch (`SceneComponent.K2_GetComponentRotation` (`Actor.GetComponentByClass` (`self.MyParent`) "/Script/Engine.CameraComponent")))))))

(fn `RecordSpawnedProjectile`
  (params (Projectile :type "Actor Object Reference"))
  ;[1 1 1] record transform
  (`KismetArrayLibrary.Array_Add` (`self.SpawnPositionProjectile`) (`Actor.GetTransform` Projectile))
  ;[1 1 1] record time
  (`KismetArrayLibrary.Array_Add` (`self.SpawnTimeProjectile`) (`self.RecordingTimer`)))

(fn `ResetPlaybackToBegining`
  (set `self.PlaybackTimer` 0.0)
  (set `self.MovementIterator` 0)
  (set `self.ProjectileItterator` 0))