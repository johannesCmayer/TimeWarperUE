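; SpawnManager runs timed rounds in which the player takes over a new character while earlier characters replay their recorded actions.
; Each interval it restarts all playbacks and, until PlayerStarts run out, spawns and possesses a FirstPersonCharacter whose RecordAndPlaybackActions component starts recording.
; A prep phase shows a red light and cone with PlayerController tick disabled, then turns green, plays a start sound and re-enables tick.
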(event `self.ReceiveBeginPlay`
  ;[1 1 1] Get spawnpoint refferences
  (bind _outactors (`GameplayStatics.GetAllActorsOfClass` "/Script/Engine.PlayerStart"))
  (set `self.PlayerSpawns` _outactors))

(event `self.ReceiveTick`
  (params (DeltaSeconds :type "Float (single-precision)"))
  ;[1 1 1] Set Timer; Check if over SpawnTime; Set new SpawnTime
  (set `self.RespawnTimer` (+ (`GameplayStatics.GetWorldDeltaSeconds`) (`self.RespawnTimer`)))
  (if (> (`self.RespawnTimer`) (`self.SpawnTime`))
    (`LightComponent.SetLightColor` (`self.PointLight`) (`KismetMathLibrary.MakeColor` 1.0) true)
    (`PrimitiveComponent.SetMaterial` (`self.Cone`) 0 "/Game/TimeWarper/Materials/RedPulsing.RedPulsing")
    (`self.SetActorTickEnabled` (`GameplayStatics.GetPlayerController` 0) false)
    (set `self.PrepTimer` 0.0)
    (set `self.SpawnTime` (+ (`self.SpawnTime`) (`self.TimeToNextSpawn`)))
    ;[1 1 1] Set all recorded players enabled and to PlayFromBegining
    (for _array_element (`self.SpawnedPlayerCharacters`)
      (`/Game/TimeWarperBP/Blueprints/Player/RecordAndPlaybackActions.PlayFromBegining` (`self.GetComponentByClass` _array_element "/Game/TimeWarperBP/Blueprints/Player/RecordAndPlaybackActions.RecordAndPlaybackActions_C"))
      (`/Game/TimeWarperBP/Blueprints/other/FunktionsAndMacros/ActorF.DisableEnableActor` _array_element))
    ;[1 1 1] Limit spawns to spawnpoint number
    (if (< (`KismetArrayLibrary.Array_Length` (`self.SpawnedPlayerCharacters`)) (`KismetArrayLibrary.Array_Length` (`self.PlayerSpawns`)))
      ;[1 1 1] Spawn player character
      (bind _returnvalue (`|SpawnActorFromClass` "/Game/TimeWarperBP/Blueprints/Player/FirstPersonCharacter.FirstPersonCharacter_C" (`self.GetTransform` (`|GetArrayItem` (`self.PlayerSpawns`) (`self.SpawnToUse`))) "Undefined" "OverrideRootScale" null null))
      (bind _result (`/Engine/EditorBlueprintResources/StandardMacros.IncrementInt` (`self.SpawnToUse`))
        (:`  `
          (set `self.SpawnToUse` _result)
          (`KismetArrayLibrary.Array_Add` (`self.SpawnedPlayerCharacters`) _returnvalue)
          (`Controller.Possess` (`GameplayStatics.GetPlayerController` 0) _returnvalue)
          ;[1 1 1] Reset all
          (for _array_element_2 (`self.SpawnedPlayerCharacters`)
            (`/Game/TimeWarperBP/Blueprints/other/FunktionsAndMacros/ActorF.DisableEnableActor` _array_element_2)
            (bind _aspawn (cast `Pawn` _array_element_2))
            (if (!= _aspawn (`Controller.K2_GetPawn` (`GameplayStatics.GetPlayerController` 0)))
              (bind _returnvalue_2 (`self.GetComponentByClass` _array_element_2 "/Game/TimeWarperBP/Blueprints/Player/RecordAndPlaybackActions.RecordAndPlaybackActions_C"))
              (`/Game/TimeWarperBP/Blueprints/Player/RecordAndPlaybackActions.PlayFromBegining` _returnvalue_2)
              (else
                (`/Game/TimeWarperBP/Blueprints/Player/RecordAndPlaybackActions.Record` _returnvalue_2)))))))
    (else
      (set `self.PrepTimer` (+ (`GameplayStatics.GetWorldDeltaSeconds`) (`self.PrepTimer`)))
      (if (> (`self.PrepTimer`) (`self.PrepTime`))
        (`AudioComponent.Play` (`self.GameStartSound`) 0.0)
        (`LightComponent.SetLightColor` (`self.PointLight`) (`KismetMathLibrary.MakeColor` 0.0 1.0) true)
        (`PrimitiveComponent.SetMaterial` (`self.Cone`) 0 "/Game/TimeWarper/Materials/GreenSimple.GreenSimple")
        (`self.SetActorTickEnabled` (`GameplayStatics.GetPlayerController` 0) true)
        (set `self.PrepTimer` -10000000000000.0)))))

(fn `UserConstructionScript`)