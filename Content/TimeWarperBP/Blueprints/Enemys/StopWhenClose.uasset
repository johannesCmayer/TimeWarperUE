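; StopWhenClose is a Behavior Tree decorator for enemy AI that gates its branch on the distance to the followed target.
; It casts the owner to EnemyAIController and reads the TargetToFollow actor from the Blackboard.
; The condition passes while the controlled pawn is at least StoppingDistance from that actor, and fails once it is closer.
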(fn `PerformConditionCheck`
  (params (OwnerActor :type "Actor Object Reference"))
  (returns (ReturnValue :type Boolean))
  (bind _asenemy_aicontroller (cast `/Game/TimeWarperBP/Blueprints/Enemys/EnemyAIController` OwnerActor))
  (set `self.EnemyAIController` _asenemy_aicontroller)
  (return (>= (`KismetMathLibrary.VSize` (- (`Actor.K2_GetActorLocation` (`BTFunctionLibrary.GetBlackboardValueAsActor` (`self.TargetToFollow`))) (`Actor.K2_GetActorLocation` (`Controller.K2_GetPawn` (`self.EnemyAIController`))))) (`self.StoppingDistance`))))