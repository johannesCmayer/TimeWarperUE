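; Behavior tree task that makes an enemy shoot at the TargetToAttack blackboard actor when it has line of sight.
; It traces on the Camera channel from the owner to the target, ignoring all EnemyAICharacter actors.
; On a hit it spawns a FirstPersonProjectile at the owner's transform and succeeds; otherwise it fails.
; The BulletSpawnOffset spawn calculation is left unconnected, and debug prints remain.
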(event `self.ReceiveExecute`
  (params (OwnerActor :type "Actor Object Reference"))
  (bind _outactors (`GameplayStatics.GetAllActorsOfClass` "/Game/TimeWarperBP/Blueprints/Enemys/EnemyAICharacter.EnemyAICharacter_C"))
  (bind _outhit (`KismetSystemLibrary.LineTraceSingle` (`Actor.K2_GetActorLocation` OwnerActor) (`Actor.K2_GetActorLocation` (`BTFunctionLibrary.GetBlackboardValueAsActor` (`self.TargetToAttack`))) "TraceTypeQuery2" false _outactors))
  (bind (_bblockinghit _binitialoverlap _time _location _impactpoint _normal _impactnormal _physmat _hitactor) (`GameplayStatics.BreakHitResult` _outhit))
  (`KismetSystemLibrary.PrintString` (`KismetSystemLibrary.GetDisplayName` _hitactor))
  (if (== _hitactor (`BTFunctionLibrary.GetBlackboardValueAsActor` (`self.TargetToAttack`)))
    (`|SpawnActorFromClass` "/Game/TimeWarperBP/Blueprints/Player/FirstPersonProjectile.FirstPersonProjectile_C" (`Actor.GetTransform` OwnerActor) "Undefined" "OverrideRootScale" null null)
    (`KismetSystemLibrary.PrintString` "AI shoots")
    (`self.FinishExecute` true)
    (else
      (`self.FinishExecute` false))))