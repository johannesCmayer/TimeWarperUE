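; AgroCheck is a behavior tree node that detects targets in sight of an enemy AI.
; Each tick it uses the cached EnemyAIController's pawn as origin for a multi-sphere object trace, ignoring all EnemyAICharacters.
; A Camera-channel line trace confirms sight to each hit, setting TargetToFollow and TargetLocation on the blackboard.
; A blocked trace clears only TargetToFollow, so the last hit checked decides the target.
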(event `self.ReceiveTick`
  (params (OwnerActor :type "Actor Object Reference") (DeltaSeconds :type "Float (single-precision)"))
  (bind _returnvalue (`Actor.K2_GetActorLocation` (`Controller.K2_GetPawn` (`self.EnemyAIController`))))
  ;[1 1 1] Check if EnemyAIController is set
  (if (not (!= (`self.EnemyAIController`) null))
    (bind _asenemy_aicontroller (cast `/Game/TimeWarperBP/Blueprints/Enemys/EnemyAIController` OwnerActor))
    (set `self.EnemyAIController` _asenemy_aicontroller))
  (bind _outactors (`GameplayStatics.GetAllActorsOfClass` "/Game/TimeWarperBP/Blueprints/Enemys/EnemyAICharacter.EnemyAICharacter_C"))
  (set `self.MyLocation` _returnvalue)
  (bind _outhits (`KismetSystemLibrary.SphereTraceMultiForObjects` _returnvalue (+ _returnvalue (0.0 0.0 15.0)) 1500.0 (`self.ObjectTypesToCheckFor`) false _outactors "None" true (struct :`R` 1.0 :`A` 1.0) (struct :`G` 1.0 :`A` 1.0) 1.0))
  (for _array_element _outhits
    (bind (_bblockinghit _binitialoverlap _time _location _impactpoint _normal _impactnormal _physmat _hitactor) (`GameplayStatics.BreakHitResult` _array_element))
    (bind _outhit (`KismetSystemLibrary.LineTraceSingle` (`self.MyLocation`) (`Actor.K2_GetActorLocation` _hitactor) "TraceTypeQuery2" false _outactors "None" true (struct :`R` 1.0 :`A` 1.0) (struct :`G` 1.0 :`A` 1.0) 1.0))
    (bind (_bblockinghit_2 _binitialoverlap_2 _time_2 _location_2 _impactpoint_2 _normal_2 _impactnormal_2 _physmat_2 _hitactor_2) (`GameplayStatics.BreakHitResult` _outhit))
    (if (== _hitactor_2 _hitactor)
      (`BTFunctionLibrary.SetBlackboardValueAsObject` (`self.TargetToFollow`) _hitactor_2)
      (`BTFunctionLibrary.SetBlackboardValueAsVector` (`self.TargetLocation`) (`Actor.K2_GetActorLocation` _hitactor_2))
      (else
        (`BTFunctionLibrary.SetBlackboardValueAsObject` (`self.TargetToFollow`))))))