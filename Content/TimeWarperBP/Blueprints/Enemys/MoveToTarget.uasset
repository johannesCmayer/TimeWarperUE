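; Behavior tree task that moves an enemy's pawn toward the actor stored in its TargetToFollow blackboard key.
; On execute it casts the owner to EnemyAIController and caches it for reuse, then runs AI MoveTo on the controlled pawn with a tight acceptance radius.
; The task finishes successfully when the move succeeds; a failed move or failed cast never calls FinishExecute.
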(event `self.ReceiveExecute`
  (params (OwnerActor :type "Actor Object Reference"))
  (if (not (!= (`self.EnemyAIController`) null))
    (bind _asenemy_aicontroller (cast `/Game/TimeWarperBP/Blueprints/Enemys/EnemyAIController` OwnerActor))
    (set `self.EnemyAIController` _asenemy_aicontroller))
  (`|AIMoveTo` (`Controller.K2_GetPawn` (`self.EnemyAIController`)) (0.0 0.0 0.0) (`BTFunctionLibrary.GetBlackboardValueAsActor` (`self.TargetToFollow`)) 5.0
    (:`OnSuccess`
      (`self.FinishExecute` true))))